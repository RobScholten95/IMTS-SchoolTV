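; Cart actor that lines up static meshes along a referenced Path spline, with a height offset and added rotation.
; Construction and BeginPlay clear the mesh and spacing arrays before looping over the emptied list to compute bounds-based spacing, then call UpdateCart.
; While Enabled, each Tick spawns every Blueprints class again, appends its mesh, and repositions all meshes.
; DistanceAlongSpline shifts the line but is never changed here.
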(event `self.ReceiveBeginPlay`
  (`|ExecutionSequence`
    (:`then_0`
      (`KismetArrayLibrary.Array_Clear` (`self.StaticMeshes`))
      (`KismetArrayLibrary.Array_Clear` (`self.ObjectY`))
      (for _array_element (`self.StaticMeshes`)
        (bind _y (.y (`.BoxExtent` (`KismetMathLibrary.BreakBoxSphereBounds` (`StaticMesh.GetBounds` (`StaticMeshComponent.StaticMesh` _array_element))))))
        (`KismetArrayLibrary.Array_Add` (`self.ObjectY`) (+ _y (.y (`self.Offset`))))
        (set `self.Offset` (`KismetMathLibrary.MakeVector` 0.0 (+ (.y (`self.Offset`)) (* _y 2.0))))))
    (:`then_1`
      (`self.UpdateCart`))))

(event `self.ReceiveTick`
  (params (DeltaSeconds :type "Float (single-precision)"))
  (if (`self.Enabled`)
    (`self.Spawn`)
    (`self.UpdateCart`)))

(event `Spawn`
  (for _array_element (`self.Blueprints`)
    (bind _returnvalue (`|SpawnActorFromClass` _array_element (`KismetMathLibrary.MakeTransform` (0.0 0.0 0.0)) "Undefined" "OverrideRootScale" null null))
    (`KismetArrayLibrary.Array_Add` (`self.StaticMeshes`) (`StaticMeshActor.StaticMeshComponent` _returnvalue))))

(event `UpdateCart`
  (bind _path (`/Game/BP_BluePrints/BP_SplinePath.Path` (`self.Path`)))
  (for (_array_element _array_index) (`self.StaticMeshes`)
    (bind _returnvalue (/ (+ (`|GetArrayItem` (`self.ObjectY`) _array_index) (`self.Distance along Spline`)) (`self.DivideOffset`)))
    (bind _returnvalue_location (`KismetMathLibrary.BreakTransform` (`KismetMathLibrary.MakeTransform` (+ (`SplineComponent.GetLocationAtDistanceAlongSpline` _path _returnvalue "World") (`KismetMathLibrary.MakeVector` 0.0 0.0 (`self.Z Offset`))))))
    (`SceneComponent.K2_SetWorldLocation` _array_element _returnvalue_location false false)
    (`SceneComponent.K2_SetWorldRotation` _array_element (`KismetMathLibrary.ComposeRotators` (`SplineComponent.GetRotationAtDistanceAlongSpline` _path _returnvalue "World") (`self.Rotation Object`)) false false)))

(fn `UserConstructionScript`
  (`|ExecutionSequence`
    (:`then_0`
      (`KismetArrayLibrary.Array_Clear` (`self.StaticMeshes`))
      (`KismetArrayLibrary.Array_Clear` (`self.ObjectY`))
      (for _array_element (`self.StaticMeshes`)
        (bind _y (.y (`.BoxExtent` (`KismetMathLibrary.BreakBoxSphereBounds` (`StaticMesh.GetBounds` (`StaticMeshComponent.StaticMesh` _array_element))))))
        (`KismetArrayLibrary.Array_Add` (`self.ObjectY`) (+ _y (.y (`self.Offset`))))
        (set `self.Offset` (`KismetMathLibrary.MakeVector` 0.0 (+ (.y (`self.Offset`)) (* _y 2.0))))))
    (:`then_1`
      (`self.UpdateCart`))))