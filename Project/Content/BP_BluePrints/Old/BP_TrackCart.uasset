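; Track cart actor, in an Old folder, that drives a train of mesh objects along a BP_SplinePath spline.
; BeginPlay creates components from ObjectArray but never adds them to ObjectsArray, whose construction-time fill is disconnected.
; While IsActive, Tick calls MoveOBJ, playing a Duration-scaled timeline that moves ObjectsArray from spline end to start.
; Each object gets an index-based distance offset, slight lift and rotation correction.
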(event `self.ReceiveBeginPlay`
  (for (_array_element _array_index) (`self.ObjectArray`)
    (`KismetSystemLibrary.PrintText` (`KismetTextLibrary.Conv_IntToText` _array_index))
    (bind _returnvalue (`AddComponent|NODE_AddStaticMeshComponent-11`))
    (`StaticMeshComponent.SetStaticMesh` _returnvalue _array_element)))

(event `self.ReceiveTick`
  (params (DeltaSeconds :type "Float (single-precision)"))
  (`GameplayStatics.GetActorOfClass` "/Game/BP_BluePrints/BP_SplinePath.BP_SplinePath_C" :!label _label)
  (if (`self.IsActive`)
    (`self.MoveOBJ`)))

(event `StartTrain`
  (goto _label))

(event `MoveOBJ`
  (bind _path (`/Game/BP_BluePrints/BP_SplinePath.Path` (`self.PathToFollow`)))
  ;[1 1 1] Setting Speed of Object
  (`TimelineComponent.SetPlayRate` (`self.TimeLineSpline`) (/ 1.0 (`self.Duration`)))
  (bind (_direction _timemoveobj) (`Timeline|TimeLineSpline`)
    (:`Update`
      (for (_array_element _array_index) (`self.ObjectsArray`)
        (bind _returnvalue (+ (`KismetMathLibrary.Lerp` (`SplineComponent.GetSplineLength` (`/Game/BP_BluePrints/BP_SplinePath.Path` (`self.PathToFollow`))) 0.0 _timemoveobj) (* _array_index (`self.Offset`))))
        (`SceneComponent.K2_SetWorldLocationAndRotation` _array_element (+ (`SplineComponent.GetLocationAtDistanceAlongSpline` _path _returnvalue "World") (0.0 0.0 5.0)) (`KismetMathLibrary.ComposeRotators` (`SplineComponent.GetRotationAtDistanceAlongSpline` _path _returnvalue "World") (struct :`Yaw` -90.0)) false false)))))

(fn `Get Offset`)

(fn `Get Size Static Mesh`
  (params (Target :type "StaticMesh Object Reference"))
  (returns (ReturnValue :type "Vector Structure"))
  (bind (_origin _boxextent) (`KismetMathLibrary.BreakBoxSphereBounds` (`StaticMesh.GetBounds` Target)))
  (return (- (+ _origin _boxextent) (- _origin _boxextent))))

(fn `UserConstructionScript`)