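; Cart actor that lays out a chain of static meshes end to end along a referenced Path spline.
; The construction script creates a component per mesh, spacing them by their bounds' Y extents, and previews the placement.
; When enabled, Tick re-samples spline location and rotation from DistanceAlongSpline, applying height and rotation offsets.
; BeginPlay optionally attaches particle systems at mesh sockets, but PausedFX deactivates only the last one spawned.
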(event `self.ReceiveBeginPlay`
  ;[1 1 1] BEGINPLAY
  (if (`self.FX Enabled`)
    (`self.SpawnFX`)))

(event `self.ReceiveTick`
  (params (DeltaSeconds :type "Float (single-precision)"))
  ;[1 1 1] TICK
  (if (`self.Enabled`)
    (`self.UpdateCart`)
    (if (`self.PausedFX`)
      (`ActorComponent.Deactivate` (`self.ParticleSystemOUT`)))))

(event `UpdateCart`
  (bind _path (`/Game/BP_BluePrints/BP_SplinePath.Path` (`self.Path`)))
  ;[1 1 1] UPDATE CART EVENT
  (for (_array_element _array_index) (`self.StaticMeshes`)
    (bind _returnvalue (/ (+ (`|GetArrayItem` (`self.ObjectY`) _array_index) (`self.Distance along Spline`)) (`self.DivideOffset`)))
    (bind _returnvalue_location (`KismetMathLibrary.BreakTransform` (`KismetMathLibrary.MakeTransform` (+ (`SplineComponent.GetLocationAtDistanceAlongSpline` _path _returnvalue "World") (`KismetMathLibrary.MakeVector` 0.0 0.0 (`self.Z Offset`))))))
    (`SceneComponent.K2_SetWorldLocation` _array_element _returnvalue_location false false)
    (`SceneComponent.K2_SetWorldRotation` _array_element (`KismetMathLibrary.ComposeRotators` (`SplineComponent.GetRotationAtDistanceAlongSpline` _path _returnvalue "World") (`self.Rotation Object`)) false false)))

(event `SpawnFX`
  ;[1 1 1] SPAWNING PARTICLE EFFECTS ON SOCKETS
  (for _array_element (`self.StaticMeshes`)
    (bind _returnvalue (`StaticMesh.FindSocket` (`StaticMeshComponent.StaticMesh` _array_element) (`self.SocketName1`)))
    (`/Engine/EditorBlueprintResources/StandardMacros.IsValid` _returnvalue
      (:`Is Valid`
        (bind _returnvalue_2 (`NiagaraFunctionLibrary.SpawnSystemAttached` (`self.Particle System`) _array_element "None" (`StaticMeshSocket.RelativeLocation` _returnvalue) (struct) "KeepRelativeOffset" false true "AutoRelease"))
        (set `self.ParticleSystemOUT` _returnvalue_2))
      (:`Is Not Valid`
        (`KismetSystemLibrary.PrintString` "Socket 1 is invalid")))))

(fn `UserConstructionScript`
  ;[1 1 1] ORIGINAL
  (`|ExecutionSequence`
    (:`then_0`
      (`KismetArrayLibrary.Array_Clear` (`self.StaticMeshes`))
      (`KismetArrayLibrary.Array_Clear` (`self.ObjectY`))
      (for _array_element (`self.Objects`)
        (bind _y (.y (`.BoxExtent` (`KismetMathLibrary.BreakBoxSphereBounds` (`StaticMesh.GetBounds` _array_element)))))
        (`KismetArrayLibrary.Array_Add` (`self.ObjectY`) (+ _y (.y (`self.Offset`))))
        (set `self.Offset` (`KismetMathLibrary.MakeVector` 0.0 (+ (.y (`self.Offset`)) (* _y 2.0))))
        (bind _returnvalue (`AddComponent|NODE_AddStaticMeshComponent-7`))
        (`StaticMeshComponent.SetStaticMesh` _returnvalue _array_element)
        (`KismetArrayLibrary.Array_Add` (`self.StaticMeshes`) _returnvalue)))
    (:`then_1`
      (`self.UpdateCart`))))